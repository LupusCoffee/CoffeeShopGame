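; BP_Test1 is a test Blueprint that logs hover, unhover and interact events to verify that they fire.
; Each event prints its name along with the display name of the InstigatorActor that triggered it.
; It has no other logic, and its construction script is empty.
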(event EventUnhover
  (params (InstigatorActor :type Actor%20Object%20Reference))
  (Development|PrintString (Utilities|String|Append "Unhover by... " (Utilities|GetDisplayName InstigatorActor))))

(event EventInteract
  (params (InstigatorActor :type Actor%20Object%20Reference))
  (Development|PrintString (Utilities|String|Append "Interact by... " (Utilities|GetDisplayName InstigatorActor))))

(event EventHover
  (params (InstigatorActor :type Actor%20Object%20Reference))
  (Development|PrintString (Utilities|String|Append "Hover by... " (Utilities|GetDisplayName InstigatorActor))))

(fn ConstructionScript)