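; BP_Test is a test interactable actor for hover highlighting and interaction.
; Hover and Unhover events turn its Highlight on and off, passing the actor's ActorType.
; Interact prints a debug string naming the instigating actor.
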(event EventUnhover
  (params (InstigatorActor :type Actor%20Object%20Reference))
  (Class|HighlightComponent|DisableHighlight (Variables|Default|GetHighlight) (Variables|Default|GetActorType)))

(event EventInteract
  (params (InstigatorActor :type Actor%20Object%20Reference))
  (Development|PrintString (Utilities|String|Append "Interact by... " (Utilities|GetDisplayName InstigatorActor)) true true "(R=1.000000,G=0.000000,B=0.047206,A=1.000000)"))

(event EventHover
  (params (InstigatorActor :type Actor%20Object%20Reference))
  (Class|HighlightComponent|EnableHighlight (Variables|Default|GetHighlight) (Variables|Default|GetActorType)))

(fn ConstructionScript)